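; Blueprint for an interactable chandelier light that toggles on and off.
; Each Interact event alternates through a FlipFlop, setting the point light's intensity and swapping a chandelier mesh material between emissive and glass to match.
; Both states play the same switch sound, and the construction script is empty.
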(event EventInteract
  (Utilities|FlowControl|FlipFlop
    (:A
      (Rendering|Components|Light|SetIntensity (Variables|Default|GetPointLight) 2.0)
      (Rendering|Material|SetMaterial (Variables|Default|Getchandelier_01) 1 "/Game/Home_Interior/Materials/Mi_Emissive_02.Mi_Emissive_02")
      (Audio|Components|Audio|Play (Variables|Default|Getsfx_switch_01) 0.0))
    (:B
      (Rendering|Components|Light|SetIntensity (Variables|Default|GetPointLight) 0.0)
      (Rendering|Material|SetMaterial (Variables|Default|Getchandelier_01) 1 "/Game/Home_Interior/Materials/Glass/Mi_Glass_03.Mi_Glass_03")
      (Audio|Components|Audio|Play (Variables|Default|Getsfx_switch_01) 0.0))))

(fn ConstructionScript)