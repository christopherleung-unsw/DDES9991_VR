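; Kitchen counter Blueprint for a showcase scene that switches its finish when interacted with.
; The Interact event drives a looping, in-order MultiGate that alternates between two material sets.
; Each set swaps several material slots on the SMKitchen mesh, changing the matte colour, the wood type, and the marble or chrome surface.
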(event EventInteract
  (bind _sm_kitchen (Variables|Default|GetSM_Kitchen))
  (bind _sm_kitchen_2 (Variables|Default|GetSM_Kitchen))
  (Utilities|FlowControl|MultiGate false true -1
    (:Out%200
      (Rendering|Material|SetMaterial _sm_kitchen 7 "/Game/Home_Interior/Materials/Mi_Matte_Color.Mi_Matte_Color")
      (Rendering|Material|SetMaterial _sm_kitchen 14 "/Game/Home_Interior/Materials/Mi_Matte_Color.Mi_Matte_Color")
      (Rendering|Material|SetMaterial _sm_kitchen 16 "/Game/_DDES9991_Showcase/Materials/Mi_Wood_Walnut.Mi_Wood_Walnut")
      (Rendering|Material|SetMaterial _sm_kitchen 1 "/Game/Home_Interior/Materials/M_Marble.M_Marble"))
    (:Out%201
      (Rendering|Material|SetMaterial _sm_kitchen_2 7 "/Game/Home_Interior/Materials/Mi_Matte_Color_02.Mi_Matte_Color_02")
      (Rendering|Material|SetMaterial _sm_kitchen_2 14 "/Game/Home_Interior/Materials/Mi_Matte_Color_02.Mi_Matte_Color_02")
      (Rendering|Material|SetMaterial _sm_kitchen_2 16 "/Game/_DDES9991_Showcase/Materials/Mi_Wood_Oak.Mi_Wood_Oak")
      (Rendering|Material|SetMaterial _sm_kitchen_2 1 "/Game/Home_Interior/Materials/Metal/M_Metal_Chrome.M_Metal_Chrome"))))

(fn ConstructionScript)