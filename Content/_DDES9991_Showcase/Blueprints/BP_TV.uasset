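; BP_TV is an interactable television that switches on and off each time it receives an Interact event.
; A FlipFlop alternates between two states: on shows the screen plane, lights a RectLight and raises the volume of a looping ambient pad sound.
; Off hides the screen and sets both the light intensity and the sound volume to zero, muting the loop without stopping it.
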(event EventInteract
  (Utilities|FlowControl|FlipFlop
    (:A
      (Development|SetHiddeninGame (Variables|Default|GetScreenPlane) false false)
      (Rendering|Components|Light|SetIntensity (Variables|Default|GetRectLight) 2.0)
      (Audio|Components|Audio|SetVolumeMultiplier (Variables|Default|Getsfx_ambient-pads-loop_01) 0.6 :!class /Script/Engine.AudioComponent))
    (:B
      (Development|SetHiddeninGame (Variables|Default|GetScreenPlane) true false)
      (Rendering|Components|Light|SetIntensity (Variables|Default|GetRectLight) 0.0)
      (Audio|Components|Audio|SetVolumeMultiplier (Variables|Default|Getsfx_ambient-pads-loop_01) 0.0 :!class /Script/Engine.AudioComponent))))

(fn ConstructionScript)