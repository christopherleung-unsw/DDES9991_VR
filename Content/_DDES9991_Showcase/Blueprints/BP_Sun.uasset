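; BP_Sun is a sun actor that rotates a directional light from two adjustable inputs, horizontal and vertical.
; On BeginPlay it stores the light's starting world rotation.
; Every tick it reapplies that rotation with offsets: SunVertical is clamped and remapped to a limited pitch swing, while SunHorizontal scales linearly into yaw.
; Roll keeps its starting value.
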(event EventBeginPlay
  ;[1 0.5 0] Get Sun Rotation Values at Start
  (Variables|Default|SetSunRotationStart (Transformation|GetWorldRotation (Variables|Default|GetDirectionalLight))))

(event EventTick
  (params (DeltaSeconds :type Float%20%28single-precision%29))
  (bind _sunrotationstart (Variables|Default|GetSunRotationStart))
  (bind (_roll _pitch _yaw) (Math|Rotator|BreakRotator _sunrotationstart))
  ;[1 0.5 0] Update Sun Rotation Values Every Tick
  (Transformation|SetWorldRotation (Variables|Default|GetDirectionalLight) (Math|Rotator|MakeRotator _roll (+ _pitch (Math|Float|MapRangeClamped (Variables|Default|GetSunVertical) -1.0 1.0 -2e+01 2e+01)) (+ _yaw (* (Variables|Default|GetSun%20Horizontal) 1.8e+02))) false false))

(fn ConstructionScript)