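; BP_KitchenIsle is an interactable kitchen island that switches between two material finishes in the showcase.
; Each Interact event drives a looping, non-random MultiGate that alternates between the two looks.
; Both branches set every targeted material slot on the island table mesh, pairing matte color, metal and oak in one look and matte color, glossy color and walnut in the other.
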(event EventInteract
  (bind _sm_kitchen_island_table (Variables|Default|GetSM_Kitchen_island_table))
  (bind _sm_kitchen_island_table_2 (Variables|Default|GetSM_Kitchen_island_table))
  (Utilities|FlowControl|MultiGate false true -1
    (:Out%200
      (Rendering|Material|SetMaterial _sm_kitchen_island_table_2 0 "/Game/Home_Interior/Materials/Mi_Matte_Color_02.Mi_Matte_Color_02")
      (Rendering|Material|SetMaterial _sm_kitchen_island_table_2 2 "/Game/Home_Interior/Materials/Mi_Matte_Color_02.Mi_Matte_Color_02")
      (Rendering|Material|SetMaterial _sm_kitchen_island_table_2 1 "/Game/Home_Interior/Materials/Metal/Mi_Metal.Mi_Metal")
      (Rendering|Material|SetMaterial _sm_kitchen_island_table_2 3 "/Game/Home_Interior/Materials/Metal/Mi_Metal.Mi_Metal")
      (Rendering|Material|SetMaterial _sm_kitchen_island_table_2 4 "/Game/_DDES9991_Showcase/Materials/Mi_Wood_Oak.Mi_Wood_Oak"))
    (:Out%201
      (Rendering|Material|SetMaterial _sm_kitchen_island_table 0 "/Game/Home_Interior/Materials/M_Matte_Color.M_Matte_Color")
      (Rendering|Material|SetMaterial _sm_kitchen_island_table 2 "/Game/Home_Interior/Materials/M_Matte_Color.M_Matte_Color")
      (Rendering|Material|SetMaterial _sm_kitchen_island_table 1 "/Game/Home_Interior/Materials/M_Glossy_Color.M_Glossy_Color")
      (Rendering|Material|SetMaterial _sm_kitchen_island_table 3 "/Game/Home_Interior/Materials/M_Glossy_Color.M_Glossy_Color")
      (Rendering|Material|SetMaterial _sm_kitchen_island_table 4 "/Game/_DDES9991_Showcase/Materials/Mi_Wood_Walnut.Mi_Wood_Walnut"))))

(fn ConstructionScript)