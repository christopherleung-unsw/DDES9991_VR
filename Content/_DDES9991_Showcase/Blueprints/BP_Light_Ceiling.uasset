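; BP_Light_Ceiling is a ceiling light that switches on and off each time its Interact event fires.
; A FlipFlop alternates the intensity of one top and two bottom lights between lit and zero, with the top dimmer when lit.
; Each toggle also swaps the lamp mesh material between emissive and copper and plays a switch sound.
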(event EventInteract
  (Utilities|FlowControl|FlipFlop
    (:A
      (Rendering|Components|Light|SetIntensity (Variables|Default|GetBottom) 2.0)
      (Rendering|Components|Light|SetIntensity (Variables|Default|GetTop) 0.5)
      (Rendering|Material|SetMaterial (Variables|Default|GetSM_Lamp_02) 0 "/Game/Home_Interior/Materials/Mi_Emissive_04.Mi_Emissive_04")
      (Audio|Components|Audio|Play (Variables|Default|Getsfx_switch_01) 0.0))
    (:B
      (Rendering|Components|Light|SetIntensity (Variables|Default|GetTop) 0.0)
      (Rendering|Material|SetMaterial (Variables|Default|GetSM_Lamp_02) 0 "/Game/StarterContent/Materials/M_Metal_Copper.M_Metal_Copper")
      (Audio|Components|Audio|Play (Variables|Default|Getsfx_switch_01) 0.0))))

(fn ConstructionScript)