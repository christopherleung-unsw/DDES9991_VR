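; BP_Light_Floor1 is an interactable floor lamp that switches on and off.
; Each Interact event runs a FlipFlop that alternates the spotlight between lit and zero intensity.
; It also swaps one material slot on the lamp mesh between emissive and glass to match, and plays a switch sound on every toggle.
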(event EventInteract
  (Utilities|FlowControl|FlipFlop
    (:A
      (Rendering|Components|Light|SetIntensity (Variables|Default|GetSpotLight) 4.0)
      (Rendering|Material|SetMaterial (Variables|Default|GetSM_Floor_lamp) 1 "/Game/Home_Interior/Materials/Mi_Emissive.Mi_Emissive")
      (Audio|Components|Audio|Play (Variables|Default|Getsfx_switch_01) 0.0))
    (:B
      (Rendering|Components|Light|SetIntensity (Variables|Default|GetSpotLight) 0.0)
      (Rendering|Material|SetMaterial (Variables|Default|GetSM_Floor_lamp) 1 "/Game/Home_Interior/Materials/Glass/Mi_Glass_02_02.Mi_Glass_02_02")
      (Audio|Components|Audio|Play (Variables|Default|Getsfx_switch_01) 0.0))))

(fn ConstructionScript)